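; BP_Radar is an early radar Blueprint that fires a debug-drawn line trace when the Fire input is pressed.
; FireTrace casts on the Visibility channel from the Arrow component along its up vector for TraceDist, without using the hit result.
; SwitchChannel is an unfinished event whose switch has no connected branches, and BeginPlay, Tick and overlap are empty.
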(event `FireTrace`
  (bind _arrow (`self.Arrow`))
  (bind _returnvalue (`SceneComponent.K2_GetComponentLocation` _arrow))
  (`KismetSystemLibrary.LineTraceSingle` :`Start` _returnvalue :`End` (+ _returnvalue (* (`KismetMathLibrary.GetUpVector` (`SceneComponent.K2_GetComponentRotation` _arrow)) (`self.TraceDist`))) :`TraceChannel` "TraceTypeQuery1" :`DrawDebugType` "ForDuration"))

(event `SwitchChannel`
  (switch `ETraceTypeQuery` "TraceTypeQuery1"))

(event `InputAction|Fire`
  (params (Key :type "Key Structure"))
  (:`Pressed`
    (`self.FireTrace`)))

(fn `UserConstructionScript`)