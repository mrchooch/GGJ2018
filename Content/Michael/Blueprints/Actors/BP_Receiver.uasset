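; BP_Receiver is an actor that catches Wave actors and checks whether each one matches its accepted type.
; On overlap with an actor tagged "Wave", it casts to Wave and compares the material on that wave's Plane to AcceptedMaterial.
; It prints GOOD or BAD as debug feedback, then destroys the wave.
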(event `self.ReceiveActorBeginOverlap`
  (params (OtherActor :type "Actor Object Reference"))
  (if (`self.ActorHasTag` OtherActor "Wave")
    (bind _aswave (cast `/Game/Tyler/Blueprints/Wave` OtherActor))
    (if (== (`PrimitiveComponent.GetMaterial` (`/Game/Tyler/Blueprints/Wave.Plane` _aswave) 0) (`self.AcceptedMaterial`))
      (`KismetSystemLibrary.PrintString` "GOOD")
      (else
        (`KismetSystemLibrary.PrintString` "BAD")))
    (`self.K2_DestroyActor` OtherActor)))

(fn `UserConstructionScript`)