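; BP_Bat is a bat pawn that wanders through the air in the YZ plane, with no movement input along X.
; On BeginPlay it picks a random direction and starts a looping timer that calls ChangeDirection periodically.
; ChangeDirection randomizes MovementVector with a narrower vertical range than horizontal, and Tick feeds that vector to the FloatingPawnMovement component as input.
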(event `self.ReceiveBeginPlay`
  (`self.ChangeDirection`)
  (`KismetSystemLibrary.K2_SetTimer` null "ChangeDirection" 10.0 true))

(event `self.ReceiveTick`
  (params (DeltaSeconds :type "Float (single-precision)"))
  (`PawnMovementComponent.AddInputVector` (`self.FloatingPawnMovement`) (`self.MovementVector`) false))

(fn `ChangeDirection`
  (set `self.MovementVector` (`KismetMathLibrary.MakeVector` 0.0 (`KismetMathLibrary.RandomFloatInRange` -1.0 1.0) (`KismetMathLibrary.RandomFloatInRange` -0.5 0.5))))

(fn `UserConstructionScript`)